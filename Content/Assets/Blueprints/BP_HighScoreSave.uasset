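; BP_HighScoreSave holds the high-score table as an array of player score structs and provides functions to query and rank it.
; GetLowestScore and GetHighestScore each scan the array linearly, returning the matching entry and its index.
; SortSaveData orders scores from highest to lowest by selection sort, repeatedly moving the top entry into a temporary array, then assigning that back to PlayerScoreSave.
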(fn `GetHighestScore`
  (returns (HighestScoreStruct :type "/Game/Assets/Structs/S_HighScoreHolder Structure") (HighestScoreIndex :type Integer))
  (locals (HighestScore :type "Float (double-precision)") (HighestIndex :type Integer))
  (bind _highestindex (`local.HighestIndex`))
  (for (_array_element _array_index) (`self.PlayerScoreSave`)
    (if (== _array_index 0)
      (set `local.HighestScore` (`.Score_5_CC5D099E4FDE474E733B50A230E37073` (break `/Game/Assets/Structs/S_HighScoreHolder` _array_element)))
      (set `local.HighestIndex` _array_index)
      (elif (> (`.Score_5_CC5D099E4FDE474E733B50A230E37073` (break `/Game/Assets/Structs/S_HighScoreHolder` _array_element)) (`local.HighestScore`))
        (set `local.HighestScore` (`.Score_5_CC5D099E4FDE474E733B50A230E37073` (break `/Game/Assets/Structs/S_HighScoreHolder` _array_element)))
        (set `local.HighestIndex` _array_index))))
  (return (`|GetArrayItem` (`self.PlayerScoreSave`) _highestindex) _highestindex))

(fn `GetLowestScore`
  (returns (LowestScoreStruct :type "/Game/Assets/Structs/S_HighScoreHolder Structure") (LowestScoreIndex :type Integer))
  (locals (LowestScore :type "Float (double-precision)") (LowestIndex :type Integer))
  (bind _lowestindex (`local.LowestIndex`))
  (for (_array_element _array_index) (`self.PlayerScoreSave`)
    (if (== _array_index 0)
      (set `local.LowestScore` (`.Score_5_CC5D099E4FDE474E733B50A230E37073` (break `/Game/Assets/Structs/S_HighScoreHolder` _array_element)))
      (set `local.LowestIndex` _array_index)
      (elif (< (`.Score_5_CC5D099E4FDE474E733B50A230E37073` (break `/Game/Assets/Structs/S_HighScoreHolder` _array_element)) (`local.LowestScore`))
        (set `local.LowestScore` (`.Score_5_CC5D099E4FDE474E733B50A230E37073` (break `/Game/Assets/Structs/S_HighScoreHolder` _array_element)))
        (set `local.LowestIndex` _array_index))))
  (return (`|GetArrayItem` (`self.PlayerScoreSave`) _lowestindex) _lowestindex))

(fn `SortSaveData`
  (locals (TempSaveStruct :type "Array of /Game/Assets/Structs/S_HighScoreHolder Structure"))
  (while (> (`KismetArrayLibrary.Array_Length` (`self.PlayerScoreSave`)) 0)
    (bind (_highestscorestruct _highestscoreindex) (`self.GetHighestScore`))
    (`KismetArrayLibrary.Array_Add` (`local.TempSaveStruct`) _highestscorestruct)
    (`KismetArrayLibrary.Array_Remove` (`self.PlayerScoreSave`) _highestscoreindex))
  (set `self.PlayerScoreSave` (`local.TempSaveStruct`)))