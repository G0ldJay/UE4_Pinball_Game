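; Pinball slingshot bumper Blueprint that kicks the ball away and awards points when a BP_Pinball overlaps it.
; On overlap it adds its Points to the score through GMB_PinballGameMode and applies a velocity-change impulse along the Capsule's forward vector.
; A SlingShotBounce timeline then drives the PercentageOut parameter on a dynamic material created in the construction script, animating the bounce through the material.
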(event `self.ReceiveActorBeginOverlap`
  (params (OtherActor :type "Actor Object Reference"))
  (bind _asbp_pinball (cast `/Game/Assets/Blueprints/BP_Pinball` OtherActor))
  (bind _asgmb_pinball_game_mode (cast `/Game/Assets/Blueprints/GMB_PinballGameMode` (`GameplayStatics.GetGameMode`)))
  (`/Game/Assets/Blueprints/GMB_PinballGameMode.AddScore` _asgmb_pinball_game_mode (`self.Points`))
  (`PrimitiveComponent.AddImpulse` (`/Game/Assets/Blueprints/BP_Pinball.Pinball` _asbp_pinball) (* (`SceneComponent.GetForwardVector` (`self.Capsule`)) 2500.0) "None" true)
  (bind (_direction _bounce) (`Timeline|SlingShotBounce` :!via `PlayFromStart`)
    (:`Update`
      (bind _asmaterial_instance_dynamic (cast `MaterialInstanceDynamic` (`PrimitiveComponent.GetMaterial` (`self.SlingShot`) 2)))
      (`MaterialInstanceDynamic.SetScalarParameterValue` _asmaterial_instance_dynamic "PercentageOut" _bounce))))

(fn `UserConstructionScript`
  (`PrimitiveComponent.CreateDynamicMaterialInstance` (`self.SlingShot`) 2 null "None"))