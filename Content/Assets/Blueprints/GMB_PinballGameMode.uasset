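; Pinball game mode that runs the game from main menu through ball play, multiplied scoring and end-of-game scoreboard.
; ResetGame restores class defaults, shows the player HUD and spawns a ball at the plunger; each destroyed ball respawns until none remain.
; EndGame opens the scoreboard only if the saved list has room or the score matches or beats its lowest.
; GetSaveGameData lazily caches the high-score save, loading and sorting it or creating a new one.
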(event `self.ReceiveBeginPlay`
  (`self.CreateMainMenuHUD`))

(event `SpawnBall`
  (bind _returnvalue (`GameplayStatics.GetActorOfClass` "/Game/Assets/Blueprints/BP_Plunger.BP_Plunger_C"))
  (bind _returnvalue_2 (`|SpawnActorFromClass` "/Game/Assets/Blueprints/BP_Pinball.BP_Pinball_C" (`KismetMathLibrary.MakeTransform` (`/Game/Assets/Blueprints/BP_Plunger.GetBallSpawnLocation` _returnvalue)) "Undefined" "OverrideRootScale" null null))
  (add `self.OnDestroyed` _returnvalue_2 (delegate `OnBallDestroyed`)))

(event `OnBallDestroyed` :!signature `self.OnDestroyed`
  (params (DestroyedActor :type "Actor Object Reference"))
  (if (> (`self.PinballsRemaining`) 0)
    (`/Engine/EditorBlueprintResources/StandardMacros.DecrementInt` (`self.PinballsRemaining`)
      (:`  `
        (`self.SpawnBall`)))
    (else
      (`self.EndGame`))))

(event `ResetGame`
  (bind (_score _multiplier _pinballsremaining) (defaults `/Game/Assets/Blueprints/GMB_PinballGameMode` "GMB_PinballGameMode_C"))
  (bind _aspc_pinball_player_controller (cast `/Game/Assets/Blueprints/PC_PinballPlayerController` (`GameplayStatics.GetPlayerController` 0) :!pure true))
  (set `self.Score` _score)
  (set `self.Multiplier` _multiplier)
  (set `self.PinballsRemaining` _pinballsremaining)
  (`self.SpawnBall`)
  (`/Game/Assets/Blueprints/PC_PinballPlayerController.CreatePlayerHUD` _aspc_pinball_player_controller)
  (set `PlayerController.bShowMouseCursor` false _aspc_pinball_player_controller))

(event `EndGame`
  (bind _currentsavegameobject (`self.GetSaveGameData`))
  (if (<= (`KismetArrayLibrary.Array_Length` (`/Game/Assets/Blueprints/BP_HighScoreSave.PlayerScoreSave` _currentsavegameobject)) (`self.ScoreboardLength`))
    (`self.CreateScoreboardHUD` :!label _label)
    (else
      (bind _lowestscorestruct (`/Game/Assets/Blueprints/BP_HighScoreSave.GetLowestScore` _currentsavegameobject))
      (if (<= (`.Score_5_CC5D099E4FDE474E733B50A230E37073` (break `/Game/Assets/Structs/S_HighScoreHolder` _lowestscorestruct)) (`self.Score`))
        (goto _label)))))

(event `CreateScoreboardHUD`
  (bind _aspc_pinball_player_controller (cast `/Game/Assets/Blueprints/PC_PinballPlayerController` (`GameplayStatics.GetPlayerController` 0) :!pure true))
  (bind _returnvalue (`|CreateWidget` "/Game/Assets/Interfaces/UI_Scoreboard.UI_Scoreboard_C" _aspc_pinball_player_controller))
  (`UserWidget.AddToViewport` _returnvalue 0)
  (set `PlayerController.bShowMouseCursor` true _aspc_pinball_player_controller))

(event `CreateMainMenuHUD`
  (bind _aspc_pinball_player_controller (cast `/Game/Assets/Blueprints/PC_PinballPlayerController` (`GameplayStatics.GetPlayerController` 0) :!pure true))
  (`self.GetSaveGameData`)
  (`WidgetLayoutLibrary.RemoveAllWidgets`)
  (bind _returnvalue (`|CreateWidget` "/Game/Assets/Interfaces/MainMenu.MainMenu_C" _aspc_pinball_player_controller))
  (`UserWidget.AddToViewport` _returnvalue 0)
  (set `PlayerController.bShowMouseCursor` true _aspc_pinball_player_controller))

(fn `AddScore`
  (params (Points :type "Float (double-precision)"))
  (returns (NewScore :type "Float (double-precision)"))
  (bind _output_get (set `self.Score` (+ (* Points (`self.Multiplier`)) (`self.Score`))))
  (return _output_get))

(fn `GetSaveGameData`
  (returns (CurrentSaveGameObject :type "/Game/Assets/Blueprints/BP_HighScoreSave Object Reference"))
  (bind _currentscoresave (`self.CurrentScoreSave`)
    (:`then`
      (return _currentscoresave))
    (:`else`
      (bind _returnvalue (`GameplayStatics.DoesSaveGameExist` (`self.HighScoreSaveName`)))
      (if _returnvalue
        (bind _returnvalue_2 (`GameplayStatics.LoadGameFromSlot` (`self.HighScoreSaveName`)))
        (bind _asbp_high_score_save (cast `/Game/Assets/Blueprints/BP_HighScoreSave` _returnvalue_2)
          (:`then`
            (`/Game/Assets/Blueprints/BP_HighScoreSave.SortSaveData` _asbp_high_score_save)
            (bind _output_get (set `self.CurrentScoreSave` _asbp_high_score_save))
            (return _output_get))
          (:`CastFailed`
            _))
        (else
          (bind _returnvalue_3 (`GameplayStatics.CreateSaveGameObject` "/Game/Assets/Blueprints/BP_HighScoreSave.BP_HighScoreSave_C"))
          (bind _asbp_high_score_save_2 (cast `/Game/Assets/Blueprints/BP_HighScoreSave` _returnvalue_3)
            (:`then`
              (bind _output_get_2 (set `self.CurrentScoreSave` _asbp_high_score_save_2))
              (return _output_get_2))
            (:`CastFailed`
              _))))
      (return null))))

(fn `UserConstructionScript`)