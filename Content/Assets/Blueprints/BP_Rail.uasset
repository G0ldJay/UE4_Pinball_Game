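; BP_Rail is a rail actor that builds its visible track from spline meshes along the SplineRail spline.
; The construction script adds one segment per pair of neighboring points, using start, middle and end meshes, with an adjustable start scale on the first.
; GetStartEndLocTan supplies each segment's local-space locations and tangents so the meshes bend along the spline.
; The event graph has no active logic.
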(fn `GetStartEndLocTan`
  (params (Spline :type "SplineComponent Object Reference") (Index :type Integer))
  (returns (`Start Location` :type "Vector Structure") (`Start Tangent` :type "Vector Structure") (`End Location` :type "Vector Structure") (`End Tangent` :type "Vector Structure"))
  (bind (_location _tangent) (`SplineComponent.GetLocationAndTangentAtSplinePoint` Spline Index "Local"))
  (bind (_location_2 _tangent_2) (`SplineComponent.GetLocationAndTangentAtSplinePoint` Spline (+ Index 1) "Local"))
  (return _location _tangent _location_2 _tangent_2))

(fn `UserConstructionScript`
  (bind _returnvalue (- (`SplineComponent.GetNumberOfSplinePoints` (`self.SplineRail`)) 2))
  (for _index (range (+ _returnvalue 1))
    (bind _returnvalue_2 (`AddComponent|NODE_AddSplineMeshComponent-0`))
    (if (== _index 0)
      (`StaticMeshComponent.SetStaticMesh` _returnvalue_2 (`self.RailStartMesh`))
      (`SplineMeshComponent.SetStartScale` _returnvalue_2 (`KismetMathLibrary.MakeVector2D` (`self.SplineStartScale`) 1.0) true)
      (elif (== _returnvalue _index)
        (`StaticMeshComponent.SetStaticMesh` _returnvalue_2 (`self.RailEndMesh`))
        (else
          (`StaticMeshComponent.SetStaticMesh` _returnvalue_2 (`self.RailMidMesh`)))))
    (bind (_start_location _start_tangent _end_location _end_tangent) (`self.GetStartEndLocTan` (`self.SplineRail`) _index))
    (`SplineMeshComponent.SetStartAndEnd` _returnvalue_2 _start_location _start_tangent _end_location _end_tangent true)))